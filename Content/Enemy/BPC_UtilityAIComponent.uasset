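; Utility AI component on an enemy's Controller that picks the enemy's next action by score.
; On BeginPlay it caches the blackboard and the controlled BP_EnemyAI.
; ChooseAction rules out actions lacking stamina or range, multiplies response-curve values of normalized enemy inputs for the rest, and returns the best action's tag.
; Scores are stored per tag in a map, which DrawHUDDebugText prints on screen.
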(event EventBeginPlay
  (bind _ascontroller (Utilities|Casting|CastToController (Components|GetOwner)))
  (Variables|Default|SetBlackBoardRef (AI|GetBlackboard _ascontroller))
  (bind _asbp_enemy_ai (Utilities|Casting|CastToBP_EnemyAI (Pawn|GetControlledPawn _ascontroller)))
  (Variables|Default|SetEnemyRef _asbp_enemy_ai))

(fn ChooseAction
  (bind _enemyref (Variables|Default|GetEnemyRef))
  (LocalVariables|SetHighestScore 0.0)
  (for _array_element (Variables|Default|GetAllActions)
    (LocalVariables|SetCurrentActionScore 1.0)
    (if (or (< (Variables|/Game/Enemy/BP_EnemyAI.BP_EnemyAI_C|GetStamina _enemyref) (.StaminaCost (Utilities|Struct|BreakS_ActionDetails (Variables|/Game/Enemy/PDA_Actions.PDA_Actions_C|GetS_Action _array_element)))) (> (Transformation|GetDistanceTo _enemyref (Variables|/Game/Enemy/BP_EnemyAI.BP_EnemyAI_C|GetPlayerRef _enemyref)) (.MaxRange (Utilities|Struct|BreakS_ActionDetails (Variables|/Game/Enemy/PDA_Actions.PDA_Actions_C|GetS_Action _array_element)))))
      (LocalVariables|SetCurrentActionScore 0.0)
      (else
        (for _array_element_2 (.Curve (Utilities|Struct|BreakS_ActionDetails (Variables|/Game/Enemy/PDA_Actions.PDA_Actions_C|GetS_Action _array_element)))
          (bind _currentvalue (Class|BPIUtilityInputs|GetInputFloat(Message) (Variables|Default|GetEnemyRef) (.InputType (Utilities|Struct|BreakS_ActionCurves _array_element_2)) _array_element))
          (LocalVariables|SetCurrentActionScore (* (LocalVariables|GetCurrentActionScore) (Math|Curves|GetFloatValue (.ResponseCurve (Utilities|Struct|BreakS_ActionCurves _array_element_2)) (Math|Float|MapRangeClamped _currentvalue (.MIn (Utilities|Struct|BreakS_ActionCurves _array_element_2)) (.Max (Utilities|Struct|BreakS_ActionCurves _array_element_2)) 0.0 1.0)))))
        (Utilities|Map|Add (Variables|Default|GetActionScoresMap) (.Tag (Utilities|Struct|BreakS_ActionDetails (Variables|/Game/Enemy/PDA_Actions.PDA_Actions_C|GetS_Action _array_element))) (LocalVariables|GetCurrentActionScore))
        (if (> (LocalVariables|GetCurrentActionScore) (LocalVariables|GetHighestScore))
          (LocalVariables|SetHighestScore (LocalVariables|GetCurrentActionScore))
          (Variables|Default|SetBest%20Action _array_element)))))
  (Utilities|IsValid (Variables|Default|GetBest%20Action)
    (:Is%20Valid
      (Development|PrintString (Utilities|String|ToString(Name) (GameplayTags|GetTagName (.Tag (Utilities|Struct|BreakS_ActionDetails (Variables|/Game/Enemy/PDA_Actions.PDA_Actions_C|GetS_Action (Variables|Default|GetBest%20Action)))))) true true "(R=0.000000,G=0.660000,B=1.000000,A=1.000000)" 2.0 "sd")
      (return (.Tag (Utilities|Struct|BreakS_ActionDetails (Variables|/Game/Enemy/PDA_Actions.PDA_Actions_C|GetS_Action (Variables|Default|GetBest%20Action))))))
    (:Is%20Not%20Valid
      (Development|PrintString "not valid")
      (return ""))))

(fn DrawHUDDebugText
  (for (_array_element _array_index) (Variables|Default|GetAllActions)
    (if (.ReturnValue (Utilities|Map|Find (Variables|Default|GetActionScoresMap) (.Tag (Utilities|Struct|BreakS_ActionDetails (Variables|/Game/Enemy/PDA_Actions.PDA_Actions_C|GetS_Action _array_element)))))
      (Development|PrintString (Utilities|String|Append "Action: " (Utilities|String|ToString(Name) (GameplayTags|GetTagName (.Tag (Utilities|Struct|BreakS_ActionDetails (Variables|/Game/Enemy/PDA_Actions.PDA_Actions_C|GetS_Action _array_element))))) " Score: " (Utilities|String|ToString(Float) (.Value (Utilities|Map|Find (Variables|Default|GetActionScoresMap) (.Tag (Utilities|Struct|BreakS_ActionDetails (Variables|/Game/Enemy/PDA_Actions.PDA_Actions_C|GetS_Action _array_element))))))) true false "(R=0.000000,G=0.660000,B=1.000000,A=1.000000)" 0.05 (Utilities|String|StringToName (Utilities|String|Append "DebugLine_" (Utilities|String|ToString(Integer) _array_index)))))))