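; Enemy AI Blueprint that sets up a character's movement speed and maintains a regenerating stamina value.
; On BeginPlay it applies MaxSpeed to the movement component's walk speed and caches the player character.
; Tick adds a fixed, frame-rate-dependent amount of Stamina, clamped to its range.
; An AIMoveTo toward the cached player exists but is unconnected, so the Blueprint itself never starts a chase.
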(event EventBeginPlay
  (Variables|/Script/Engine.CharacterMovementComponent|SetMaxWalkSpeed (Variables|Character|GetCharacterMovement) (Variables|Default|GetMaxSpeed))
  (Variables|Default|SetPlayerRef (Game|GetPlayerCharacter 0)))

(event Collision|EventActorBeginOverlap
  (params (OtherActor :type Actor%20Object%20Reference)))

(event EventTick
  (params (DeltaSeconds :type Float%20%28single-precision%29))
  (Variables|Default|SetStamina (Math|Float|Clamp(Float) (+ (Variables|Default|GetStamina) 0.05) 0.0 1e+02)))

(fn ConstructionScript)