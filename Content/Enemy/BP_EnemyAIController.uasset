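; Enemy AI controller that runs the BT_Enemy behavior tree on possession and feeds it perception results.
; When AI Perception successfully senses the player pawn, it writes that actor to the TargetActor blackboard key and sets HasLineOfSight? true.
; Successfully sensing any other actor sets HasLineOfSight? false.
; Failed stimuli, including loss of the player, leave the blackboard unchanged.
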(event OnTargetPerceptionUpdated(AIPerception)
  (params (Actor :type Actor%20Object%20Reference) (Stimulus :type AI%20Stimulus%20Structure))
  (if (.bSuccessfullySensed (Utilities|Struct|BreakAIStimulus Stimulus))
    (if (== Actor (Game|Player|GetPlayerPawn 0))
      (AI|Components|Blackboard|SetValueasObject (Variables|Default|GetBlackboard) (Utilities|Name|MakeLiteralName "TargetActor") Actor)
      (AI|Components|Blackboard|SetValueasBool (Variables|Default|GetBlackboard) (Utilities|Name|MakeLiteralName "HasLineOfSight?") true)
      (else
        (AI|Components|Blackboard|SetValueasBool (Variables|Default|GetBlackboard) (Utilities|Name|MakeLiteralName "HasLineOfSight?") false)))))

(event EventPossess
  (params (PossessedPawn :type Pawn%20Object%20Reference))
  (AI|RunBehaviorTree "/Game/Enemy/BehaviourTree/BT_Enemy.BT_Enemy"))

(fn ConstructionScript)